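; Interactible suction cup (ventouse) actor that changes material while the first-person character overlaps it.
; Begin overlap swaps the mesh's first material to the projectile material, and end overlap restores its base color material.
; BeginPlay sets an IsPositive flag, which no logic in this Blueprint reads.
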(event `self.ReceiveActorBeginOverlap`
  (params (OtherActor :type "Actor Object Reference"))
  (cast `/Game/FirstPerson/Blueprints/BP_FirstPersonCharacter` OtherActor)
  (`PrimitiveComponent.SetMaterial` (`self.SM_VENTOUSE`) 0 "/Game/FPWeapon/Materials/FirstPersonProjectileMaterial.FirstPersonProjectileMaterial"))

(event `self.ReceiveActorEndOverlap`
  (params (OtherActor :type "Actor Object Reference"))
  (cast `/Game/FirstPerson/Blueprints/BP_FirstPersonCharacter` OtherActor)
  (`PrimitiveComponent.SetMaterial` (`self.SM_VENTOUSE`) 0 "/Game/3D/M_Ventouse_BaseColor.M_Ventouse_BaseColor"))

(event `self.ReceiveBeginPlay`
  (set `self.IsPositive` true))

(fn `UserConstructionScript`
  (`parent.UserConstructionScript`))